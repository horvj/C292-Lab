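; BP_ColorLight is a point light actor that switches between its base color and green when a linked pressure plate is pressed.
; On BeginPlay it applies the base color, picks a BP_PressurePlate from all in the level using ListenerKey as array index, and binds to its OnButtonPressed event.
; Each press toggles the color through a "Red"/"Green" string state, provided ListenerKey matches that plate's EmitterKey.
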(event Custom|ToggleColor
  (if (== (Variables|Default|GetListenerKey) (Variables|/Game/BP_PressurePlate.BP_PressurePlate_C|GetEmitterKey (Variables|Default|GetEmitterRef)))
    (if (Utilities|Enum|Equal(Enum) (Variables|Default|GetString) "Red")
      (Rendering|Components|Light|SetLightColor (Variables|Default|GetPointLight) "(R=0.197131,G=1.000000,B=0.000000,A=1.000000)" true)
      (Variables|Default|SetString "Green")
      (else
        (Rendering|Components|Light|SetLightColor (Variables|Default|GetPointLight) (Variables|Default|GetBaseLightColor) true)
        (Variables|Default|SetString "Red")))
    (Utilities|FlowControl|Delay 2.0)))

(event EventBeginPlay
  (Variables|Default|SetString "Red")
  (bind _outactors (Actor|GetAllActorsOfClass "/Game/BP_PressurePlate.BP_PressurePlate_C"))
  (Rendering|Components|Light|SetLightColor (Variables|Default|GetPointLight) (Variables|Default|GetBaseLightColor) true)
  (Variables|Default|SetEmitterRef (Utilities|Array|Get(acopy) _outactors (Variables|Default|GetListenerKey)))
  (EventDispatchers|BindEventtoOnButtonPressed (Utilities|Array|Get(acopy) _outactors (Variables|Default|GetListenerKey)) (delegate Custom|ToggleColor)))

(fn ConstructionScript)