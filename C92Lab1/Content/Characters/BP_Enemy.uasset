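; Enemy character that chases the first-person player and destroys any "Player"-tagged actor that overlaps its capsule.
; Tick continually issues AI MoveTo toward the player's pawn.
; Actor overlap and capsule hit share death logic that checks for a "Bullet" tag, sets ShouldDie, spawns a BP_Key, then destroys the enemy after a short delay.
; Death montage nodes are left unconnected, and a debug "Hello" print remains.
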(event OnComponentHit(CapsuleComponent)
  (params (HitComponent :type Primitive%20Component%20Object%20Reference) (OtherActor :type Actor%20Object%20Reference) (OtherComp :type Primitive%20Component%20Object%20Reference) (NormalImpulse :type Vector :default "0, 0, 0") (Hit :type Hit%20Result%20Structure%20%28by%20ref%29))
  (Development|PrintString "Hello")
  (if (Actor|ActorHasTag (stale Collision|EventActorBeginOverlap OtherActor) "Bullet")
    (Variables|Default|SetshouldDie true)
    (Game|SpawnActorfromClass "/Game/Key/BP_Key.BP_Key_C" (Transformation|GetActorTransform self) "Undefined" "MultiplyWithRoot" 0 0)
    (Utilities|FlowControl|Delay 1.0)
    (Actor|DestroyActor)))

(event OnComponentBeginOverlap(CapsuleComponent)
  (params (OverlappedComponent :type Primitive%20Component%20Object%20Reference) (OtherActor :type Actor%20Object%20Reference) (OtherComp :type Primitive%20Component%20Object%20Reference) (OtherBodyIndex :type Integer) (bFromSweep :type Boolean) (SweepResult :type Hit%20Result%20Structure%20%28by%20ref%29))
  (if (Actor|ActorHasTag OtherActor "Player")
    (Actor|DestroyActor OtherActor)))

(event EventBeginPlay)

(event Collision|EventActorBeginOverlap
  (params (OtherActor :type Actor%20Object%20Reference))
  (Development|PrintString "Hello")
  (if (Actor|ActorHasTag OtherActor "Bullet")
    (Variables|Default|SetshouldDie true)
    (Game|SpawnActorfromClass "/Game/Key/BP_Key.BP_Key_C" (Transformation|GetActorTransform self) "Undefined" "MultiplyWithRoot" 0 0)
    (Utilities|FlowControl|Delay 1.0)
    (Actor|DestroyActor)))

(event EventTick
  (params (DeltaSeconds :type Float%20%28single-precision%29))
  (bind _asbp_first_person_character (Utilities|Casting|CastToBP_FirstPersonCharacter (Game|Player|GetPlayerPawn 0)))
  (AI|AIMoveTo self (Transformation|GetActorLocation _asbp_first_person_character) _asbp_first_person_character 1.0 false))

(event Collision|EventHit
  (params (MyComp :type Primitive%20Component%20Object%20Reference) (Other :type Actor%20Object%20Reference) (OtherComp :type Primitive%20Component%20Object%20Reference) (bSelfMoved :type Boolean) (HitLocation :type Vector :default "0, 0, 0") (HitNormal :type Vector :default "0, 0, 0") (NormalImpulse :type Vector :default "0, 0, 0") (Hit :type Hit%20Result%20Structure%20%28by%20ref%29)))

(fn ConstructionScript)