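; BP_Box is an actor whose Cube mesh swaps material in response to a pressure plate.
; On BeginPlay it indexes all BP_PressurePlate actors by ListenerKey and binds ToggleMaterial to that plate's OnButtonPressed dispatcher.
; When the plate's EmitterKey matches ListenerKey, the event alternates between grimy and tiled concrete, tracking state in a string and ending with a Delay that triggers nothing.
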(event Custom|ToggleMaterial
  (if (== (Variables|Default|GetListenerKey) (Variables|/Game/BP_PressurePlate.BP_PressurePlate_C|GetEmitterKey (Variables|Default|GetEmitterRef)))
    (if (Utilities|Enum|Equal(Enum) (Variables|Default|GetString) "MatOne")
      (Rendering|Material|SetMaterial (Variables|Default|GetCube) 0 "/Game/StarterContent/Materials/M_Concrete_Grime.M_Concrete_Grime")
      (Variables|Default|SetString "MatTwo")
      (else
        (Rendering|Material|SetMaterial (Variables|Default|GetCube) 0 "/Game/StarterContent/Materials/M_Concrete_Tiles.M_Concrete_Tiles")
        (Variables|Default|SetString "MatOne")))
    (Utilities|FlowControl|Delay 2.0)))

(event EventBeginPlay
  (bind _outactors (Actor|GetAllActorsOfClass "/Game/BP_PressurePlate.BP_PressurePlate_C"))
  (Variables|Default|SetEmitterRef (Utilities|Array|Get(acopy) _outactors (Variables|Default|GetListenerKey)))
  (EventDispatchers|BindEventtoOnButtonPressed (Utilities|Array|Get(acopy) _outactors (Variables|Default|GetListenerKey)) (delegate Custom|ToggleMaterial)))

(event Collision|EventActorBeginOverlap
  (params (OtherActor :type Actor%20Object%20Reference)))

(event EventTick
  (params (DeltaSeconds :type Float%20%28single-precision%29)))

(fn ConstructionScript)