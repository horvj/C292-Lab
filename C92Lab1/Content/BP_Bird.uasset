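; BP_Bird is a child Blueprint for a bird that demonstrates inherited behavior and overrides through debug print messages.
; On BeginPlay it calls the parent, then Fly, which prints a yellow message when CanFly is true.
; Its Move override calls the parent version and adds a flight message, though this graph never calls it.
; Tick triggers the Gaming event, printing a joke string every frame.
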(event EventBeginPlay
  (|CallParentFunction)
  (CallFunction|Fly (Variables|Default|GetcanFly)))

(event Collision|EventActorBeginOverlap
  (params (OtherActor :type Actor%20Object%20Reference))
  (|CallParentFunction OtherActor) ; This node is disabled and will not be called.\nDrag off pins to build functionality.
)

(event EventTick
  (params (DeltaSeconds :type Float%20%28single-precision%29))
  (|CallParentFunction DeltaSeconds)
  (CallFunction|Gaming))

(event EventGaming
  (Development|PrintString "I am a gamer"))

(fn ConstructionScript
  (|CallParentFunction))

(fn Move
  (|CallParentFunction)
  (Development|PrintString "A Bird Flies"))

(fn Fly
  (params (canFly :type Boolean))
  (if canFly
    (Development|PrintString "Flying" true true "(R=0.975856,G=1.000000,B=0.000000,A=1.000000)")))