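; BP_TriggerZone is an actor with a point light that other logic can animate and reset through Move and Stop events.
; Move plays a timeline driving pitch and yaw and turns the light red; Stop halts it, restores the BeginPlay transform and turns the light green.
; Player overlap sets CanRotate, but end overlap checks the actor's own tag, and the 1 key only prints before an empty CanRotate branch.
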(event Custom|Move
  (bind (_direction _x _y) (Timeline|Moving Play)
    (:Update
      (Transformation|SetActorRotation (Math|Rotator|MakeRotator 0.0 _x _y))
      (Rendering|Components|Light|SetLightColor (Variables|Default|GetPointLight) "(R=1.000000,G=0.000000,B=0.008376,A=1.000000)" true))))

(event Custom|Stop
  (Rendering|Components|Light|SetLightColor (Variables|Default|GetPointLight) "(R=0.000000,G=1.000000,B=0.250000,A=1.000000)" true)
  (Transformation|SetActorTransform (Variables|Default|GetInitialTransform))
  (bind (_direction _x _y) (Timeline|Moving Stop)
    (:Update
      (Transformation|SetActorRotation (Math|Rotator|MakeRotator 0.0 _x _y))
      (Rendering|Components|Light|SetLightColor (Variables|Default|GetPointLight) "(R=1.000000,G=0.000000,B=0.008376,A=1.000000)" true))))

(event EventBeginPlay
  (Variables|Default|SetInitialTransform (Transformation|GetActorTransform self)))

(event Collision|EventActorBeginOverlap
  (params (OtherActor :type Actor%20Object%20Reference))
  (if (Actor|ActorHasTag OtherActor "Player")
    (Variables|Default|SetcanRotate true)))

(event Collision|EventActorEndOverlap
  (params (OtherActor :type Actor%20Object%20Reference))
  (if (Actor|ActorHasTag "Player")
    (Variables|Default|SetcanRotate false)))

(event EventTick
  (params (DeltaSeconds :type Float%20%28single-precision%29)))

(event Input|KeyboardEvents|1
  (params (Key :type Key%20Structure :default "None"))
  (:Pressed
    (Development|PrintString "Hello")
    (if (Variables|Default|GetcanRotate)
      _)))

(fn ConstructionScript)