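; BP_Kangaroo is a kangaroo child Blueprint that reports its movement and jump ability through debug text.
; On BeginPlay it runs the parent logic, then calls Jump with its JumpHeight, which prints that height in feet in colored text.
; Its Move override calls the parent version before printing that the kangaroo walks, and nothing in this graph calls it.
; Neither function contains actual movement logic beyond that parent call.
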(event EventBeginPlay
  (|CallParentFunction)
  (CallFunction|Jump (Variables|Default|GetjumpHeight)))

(event Collision|EventActorBeginOverlap
  (params (OtherActor :type Actor%20Object%20Reference))
  (|CallParentFunction OtherActor) ; This node is disabled and will not be called.\nDrag off pins to build functionality.
)

(event EventTick
  (params (DeltaSeconds :type Float%20%28single-precision%29))
  (|CallParentFunction DeltaSeconds) ; This node is disabled and will not be called.\nDrag off pins to build functionality.
)

(fn ConstructionScript
  (|CallParentFunction))

(fn Move
  (|CallParentFunction)
  (Development|PrintString "Kangaroo Walks"))

(fn Jump
  (params (jumpHeight :type Float%20%28double-precision%29))
  (Development|PrintString (Utilities|String|Append "Can Jump: " (Utilities|String|ToString(Float) jumpHeight) " feet") true true "(R=1.000000,G=0.000000,B=0.794729,A=1.000000)"))