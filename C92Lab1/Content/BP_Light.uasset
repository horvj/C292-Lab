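; BP_Light is an actor whose point light starts hidden and toggles when a linked BP_PressurePlate is pressed.
; On BeginPlay it uses ListenerKey as an index into all pressure plates in the level, stores that plate and binds to its OnButtonPressed event.
; ToggleLight flips the light only if the plate's EmitterKey equals ListenerKey, then ends on a delay that drives nothing.
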(event Custom|ToggleLight
  (if (== (Variables|Default|GetListenerKey) (Variables|/Game/BP_PressurePlate.BP_PressurePlate_C|GetEmitterKey (Variables|Default|GetEmitterReference)))
    (if (Rendering|IsVisible (Variables|Default|GetPointLight))
      (Development|SetHiddeninGame (Variables|Default|GetPointLight) true false)
      (else
        (Development|SetHiddeninGame (Variables|Default|GetPointLight) false false)))
    (Utilities|FlowControl|Delay 2.0)))

(event EventBeginPlay
  (bind _outactors (Actor|GetAllActorsOfClass "/Game/BP_PressurePlate.BP_PressurePlate_C"))
  (Development|SetHiddeninGame (Variables|Default|GetPointLight) true false)
  (Variables|Default|SetEmitterReference (Utilities|Array|Get(acopy) _outactors (Variables|Default|GetListenerKey)))
  (EventDispatchers|BindEventtoOnButtonPressed (Utilities|Array|Get(acopy) _outactors (Variables|Default|GetListenerKey)) (delegate Custom|ToggleLight)))

(fn ConstructionScript)